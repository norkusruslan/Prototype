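; Player controller that turns the controlled pawn to face the mouse cursor.
; Each tick it deprojects the mouse position into a world ray from the camera location and intersects it with a plane through the pawn's location.
; When the intersection succeeds, it applies only the yaw of the look-at rotation from the pawn to that point.
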(event `self.ReceiveTick`
  (params (DeltaSeconds :type "Float (single-precision)"))
  (bind (_locationx _locationy) (`self.GetMousePosition`))
  (bind _returnvalue (`self.K2_GetPawn`))
  (bind (_returnvalue_2 _intersectionpoint) (`/Game/Blueprints/Functions/RayToPlaneIntersection.FindRayToPlaneIntersection` (`PlayerCameraManager.GetCameraLocation` (`GameplayStatics.GetPlayerCameraManager` 0)) (`.WorldDirection` (`GameplayStatics.DeprojectScreenToWorld` self (`KismetMathLibrary.MakeVector2D` _locationx _locationy))) (0.0 0.0 0.0) (`self.K2_GetActorLocation` (`self.K2_GetPawn`))))
  (bind (_returnvalue_roll _returnvalue_pitch _returnvalue_yaw) (`KismetMathLibrary.BreakRotator` (`KismetMathLibrary.FindLookAtRotation` (`self.K2_GetActorLocation` _returnvalue) _intersectionpoint)))
  (if _returnvalue_2
    (`self.K2_SetActorRotation` _returnvalue (`KismetMathLibrary.MakeRotator` 0.0 0.0 _returnvalue_yaw) false)))

(fn `UserConstructionScript`)